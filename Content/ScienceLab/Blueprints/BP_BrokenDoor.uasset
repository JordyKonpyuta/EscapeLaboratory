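; BP_BrokenDoor is a two-panel sliding lab door that opens when something overlaps its Collision component.
; Beginning an overlap plays a timeline whose Doors track slides LabDoor03A and LabDoor03B apart along relative Y in opposite directions.
; Ending an overlap reverses the timeline to close them, with no filter on the overlapping actor.
; Tick branches on an Open variable but performs no action.
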(event OnComponentBeginOverlap(Collision)
  (params (OverlappedComponent :type Primitive%20Component%20Object%20Reference) (OtherActor :type Actor%20Object%20Reference) (OtherComp :type Primitive%20Component%20Object%20Reference) (OtherBodyIndex :type Integer) (bFromSweep :type Boolean) (SweepResult :type Hit%20Result%20Structure%20%28by%20ref%29))
  ;[0 0.3281 0] SecurityBreach0X00CF52
  (bind _doors (Timeline|Timeline Play)
    (:Update
      (Transformation|SetRelativeLocation (Variables|Default|GetLabDoor03B) (Math|Vector|MakeVector 0.0 (* _doors 1.2e+02) 0.0) false false)
      (Transformation|SetRelativeLocation (Variables|Default|GetLabDoor03A) (Math|Vector|MakeVector 0.0 (* _doors -1.2e+02) 0.0) false false))))

(event OnComponentEndOverlap(Collision)
  (params (OverlappedComponent :type Primitive%20Component%20Object%20Reference) (OtherActor :type Actor%20Object%20Reference) (OtherComp :type Primitive%20Component%20Object%20Reference) (OtherBodyIndex :type Integer))
  ;[0 0.3281 0] SecurityBreach0X00CF52
  (bind _doors (Timeline|Timeline Reverse)
    (:Update
      (Transformation|SetRelativeLocation (Variables|Default|GetLabDoor03B) (Math|Vector|MakeVector 0.0 (* _doors 1.2e+02) 0.0) false false)
      (Transformation|SetRelativeLocation (Variables|Default|GetLabDoor03A) (Math|Vector|MakeVector 0.0 (* _doors -1.2e+02) 0.0) false false))))

(event EventBeginPlay
  ;[0 0.3281 0] SecurityBreach0X00CF52
)

(event Collision|EventActorBeginOverlap
  (params (OtherActor :type Actor%20Object%20Reference))
  ;[0 0.3281 0] SecurityBreach0X00CF52
)

(event EventTick
  (params (DeltaSeconds :type Float%20%28single-precision%29))
  ;[0 0.3281 0] SecurityBreach0X00CF52
  (if (Variables|Default|GetOpen)
    _))

(fn ConstructionScript)