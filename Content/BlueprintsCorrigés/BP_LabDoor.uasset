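; BP_LabDoor is a sliding lab door that opens while a BP_Body actor is in its Collision volume.
; Begin and end overlap play and reverse a Timeline that drives the door mesh's relative Y location.
; The construction script offsets the door by DoorPosition and picks its mesh from DoorMesh, applying two materials to door and jamb, except in the variant that also swaps the jamb mesh.
; An AC_0X00A21E component call is left unconnected.
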(event OnComponentEndOverlap(Collision)
  (params (OverlappedComponent :type Primitive%20Component%20Object%20Reference) (OtherActor :type Actor%20Object%20Reference) (OtherComp :type Primitive%20Component%20Object%20Reference) (OtherBodyIndex :type Integer))
  (Utilities|Casting|CastToBP_Body OtherActor)
  ;[1 0 0] FatalCodeDoor42
  (bind _door (Timeline|Timeline Reverse)
    (:Update
      (Transformation|SetRelativeLocation (Variables|Default|GetLabDoor01) (Math|Vector|MakeVector 0.0 (* _door 1.2e+02) 0.0) false false))))

(event OnComponentBeginOverlap(Collision)
  (params (OverlappedComponent :type Primitive%20Component%20Object%20Reference) (OtherActor :type Actor%20Object%20Reference) (OtherComp :type Primitive%20Component%20Object%20Reference) (OtherBodyIndex :type Integer) (bFromSweep :type Boolean) (SweepResult :type Hit%20Result%20Structure%20%28by%20ref%29))
  ;[1 0 0] FatalCodeDoor42
  (Utilities|Casting|CastToBP_Body OtherActor)
  (bind _door (Timeline|Timeline Play)
    (:Update
      (Transformation|SetRelativeLocation (Variables|Default|GetLabDoor01) (Math|Vector|MakeVector 0.0 (* _door 1.2e+02) 0.0) false false))))

(fn ConstructionScript
  (bind _labdoor01 (Variables|Default|GetLabDoor01))
  (bind _labdoorjamb01 (Variables|Default|GetLabDoorjamb01))
  ;[1 1 1] Movement
  (Transformation|AddRelativeLocation _labdoor01 (Math|Vector|MakeVector 0.0 (Variables|Default|GetDoorPosition) 0.0) false false)
  ;[1 1 1] Change Door Mesh
  (switch int (Variables|Default|GetDoor%20Mesh)
    (:Default
      (Components|StaticMesh|SetStaticMesh _labdoor01 "/Game/ScienceLab/Meshes/Rooms/Doors/SM_LabDoor01.SM_LabDoor01" :!label _label)
      ;[1 1 1] Materail
      (Rendering|Material|SetMaterial _labdoor01 0 (Variables|Default|GetMaterail1) :!label _label_2)
      (Rendering|Material|SetMaterial _labdoorjamb01 1 (Variables|Default|GetMaterail2)))
    (:0
      (goto _label))
    (:1
      (Components|StaticMesh|SetStaticMesh _labdoor01 "/Game/ScienceLab/Meshes/Rooms/Doors/SM_LabDoor04.SM_LabDoor04")
      (goto _label_2))
    (:2
      (Components|StaticMesh|SetStaticMesh _labdoor01 "/Game/ScienceLab/Meshes/Rooms/Doors/SM_LabDoor02.SM_LabDoor02")
      (Components|StaticMesh|SetStaticMesh _labdoorjamb01 "/Game/ScienceLab/Meshes/Rooms/Doors/SM_LabDoorjamb02.SM_LabDoorjamb02"))))